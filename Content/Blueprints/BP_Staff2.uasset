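; BP_Staff2 is a holdable staff the first-person player can pick up, drop and use to turn surfaces green.
; Pick-up plays a sound and disables mesh collision, while drop restores collision, enables physics and launches it with a fixed world-axis impulse.
; Use line-traces from the hand hold point along the camera's forward vector and swaps the hit component's first material to green with a magic sound, unless already green.
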(event EventBeginPlay)

(event Collision|EventActorBeginOverlap
  (params (OtherActor :type Actor%20Object%20Reference)))

(event EventTick
  (params (DeltaSeconds :type Float%20%28single-precision%29)))

(event EventPickUp
  (params (Owner :type BPC%20Interact%20Object%20Reference))
  (Utilities|Casting|CastToBP_FirstPersonCharacter (Game|GetPlayerCharacter 0))
  (Audio|PlaySound2D "/Game/Audio/KeyPickup.KeyPickup" 1.0 1.0 0.0 0 0)
  (Collision|SetCollisionEnabled (Variables|Default|GetStaticMesh) "NoCollision"))

(event EventDrop
  (Collision|SetCollisionEnabled (Variables|Default|GetStaticMesh) "QueryAndPhysics")
  (Physics|SetSimulatePhysics (Variables|Default|GetStaticMesh) true)
  (Physics|AddImpulse (Variables|Default|GetStaticMesh) "2000.000000,0.000000,50.000000" "None" true))

(event EventUse
  (bind _asbp_first_person_character (Utilities|Casting|CastToBP_FirstPersonCharacter (Game|GetPlayerCharacter 0)))
  (bind _outhit (Collision|LineTraceByChannel (Transformation|GetWorldLocation (Variables|/Game/FirstPerson/Blueprints/BP_FirstPersonCharacter.BP_FirstPersonCharacter_C|GetHandHoldPoint _asbp_first_person_character)) (+ (* (Math|Vector|GetForwardVector (Variables|/Game/FirstPerson/Blueprints/BP_FirstPersonCharacter.BP_FirstPersonCharacter_C|GetFirstPersonCamera _asbp_first_person_character)) 1e+03) (Transformation|GetWorldLocation (Variables|/Game/FirstPerson/Blueprints/BP_FirstPersonCharacter.BP_FirstPersonCharacter_C|GetHandHoldPoint _asbp_first_person_character))) "TraceTypeQuery1" false 0 "ForDuration"))
  (if (not (== (Rendering|Material|GetMaterial (.HitComponent (Collision|BreakHitResult _outhit)) 0) "/Game/SimpleMaterials/MI_Green.MI_Green"))
    (Audio|PlaySound2D "/Game/Audio/Magic_Cue.Magic_Cue" 1.0 1.0 0.0 0 0)
    (Rendering|Material|SetMaterial (.HitComponent (Collision|BreakHitResult _outhit)) 0 "/Game/SimpleMaterials/MI_Green.MI_Green")))

(fn ConstructionScript)