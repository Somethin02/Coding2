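; Shopkeeper actor that shows a shop menu while the first-person player is within its sphere trigger.
; On BeginPlay it creates one W_ShopkeepMenu, passing in Inventory and BPCInventory, and caches it as TransferMenu.
; Entering the sphere adds the menu to the viewport and calls ShowInventory on the player.
; Leaving removes only the menu, with no matching call to hide the player's inventory.
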(event OnComponentBeginOverlap(Sphere)
  (params (OverlappedComponent :type Primitive%20Component%20Object%20Reference) (OtherActor :type Actor%20Object%20Reference) (OtherComp :type Primitive%20Component%20Object%20Reference) (OtherBodyIndex :type Integer) (bFromSweep :type Boolean) (SweepResult :type Hit%20Result%20Structure%20%28by%20ref%29))
  (bind _asbp_first_person_character (Utilities|Casting|CastToBP_FirstPersonCharacter OtherActor))
  (bind _transfermenu (Variables|Default|GetTransferMenu)
    (:then
      (UserInterface|Viewport|AddtoViewport _transfermenu 0)
      (Default|ShowInventory _asbp_first_person_character))
    (:else)))

(event OnComponentEndOverlap(Sphere)
  (params (OverlappedComponent :type Primitive%20Component%20Object%20Reference) (OtherActor :type Actor%20Object%20Reference) (OtherComp :type Primitive%20Component%20Object%20Reference) (OtherBodyIndex :type Integer))
  (Utilities|Casting|CastToBP_FirstPersonCharacter OtherActor)
  (bind _transfermenu (Variables|Default|GetTransferMenu)
    (:then
      (Widget|RemovefromParent _transfermenu))
    (:else)))

(event EventBeginPlay
  (bind _returnvalue (UserInterface|CreateWidget "/Game/Widgets/W_ShopkeepMenu.W_ShopkeepMenu_C" 0 (Variables|Default|GetInventory) (Variables|Default|GetBPC_Inventory)))
  (Variables|Default|SetTransferMenu _returnvalue))

(event Collision|EventActorBeginOverlap
  (params (OtherActor :type Actor%20Object%20Reference)))

(event EventTick
  (params (DeltaSeconds :type Float%20%28single-precision%29)))

(fn ConstructionScript)