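; BP_PurplePotion is a speed potion item that the first-person character can pick up, drop or drink.
; PickUp plays a sound, disables the mesh's collision and returns its item type.
; Drop restores collision, enables physics and launches it along a fixed world-space vector.
; Use plays a random gulp, hides the potion and briefly boosts walk speed, then resets it to a hard-coded value and destroys the actor.
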(event EventBeginPlay)

(event Collision|EventActorBeginOverlap
  (params (OtherActor :type Actor%20Object%20Reference)))

(event EventDrop
  (Collision|SetCollisionEnabled (Variables|Default|GetPotion) "QueryAndPhysics")
  (Physics|SetSimulatePhysics (Variables|Default|GetPotion) true)
  (Physics|AddImpulse (Variables|Default|GetPotion) "2000.000000,0.000000,50.000000" "None" true))

(event EventUse
  (Audio|PlaySound2D (.OutItem (Utilities|Array|Random (Variables|Default|GetGulpSounds))) 1.0 1.0 0.0 0 0)
  (bind _asbp_first_person_character (Utilities|Casting|CastToBP_FirstPersonCharacter (Game|GetPlayerCharacter 0)))
  (Variables|/Script/Engine.CharacterMovementComponent|SetMaxWalkSpeed (Variables|/Script/Engine.Character|GetCharacterMovement _asbp_first_person_character) 4e+03)
  (Rendering|SetVisibility (Variables|Default|GetPotion) false false)
  (Utilities|FlowControl|Delay 3.0)
  (Variables|/Script/Engine.CharacterMovementComponent|SetMaxWalkSpeed (Variables|/Script/Engine.Character|GetCharacterMovement _asbp_first_person_character) 6e+02)
  (Actor|DestroyActor))

(fn ConstructionScript)

(fn PickUp
  (params (Owner :type BPC%20Interact%20Object%20Reference))
  (Utilities|Casting|CastToBP_FirstPersonCharacter (Game|GetPlayerCharacter 0))
  (Audio|PlaySound2D "/Game/Audio/KeyPickup.KeyPickup" 1.0 1.0 0.0 0 0)
  (Collision|SetCollisionEnabled (Variables|Default|GetPotion) "NoCollision")
  (return (Variables|Default|GetItemType)))