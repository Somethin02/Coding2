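; Player stats component that tracks health, stamina and leveled experience, and drives a W_Stats HUD widget it creates on BeginPlay.
; Each stat is packed into a vector with Z as current value, and setters treat -1 as "keep existing".
; ChangeXP loops through level-ups and level-downs, doubling or halving the threshold.
; Health reaching zero fades the camera to red and reloads the level; stamina change and set functions are empty stubs.
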(event Custom|Death
  (Utilities|FlowControl|DoOnce false
    (:Completed
      (CameraFades|StartCameraFade (Game|GetPlayerCameraManager 0) 0.0 1.0 1.0 "(R=1.000000,G=0.000000,B=0.000000,A=1.000000)" false true)
      (Utilities|FlowControl|Delay 1.5)
      (Development|PrintString "u r dead, not big surprise")
      (bind _returnvalue (Game|GetCurrentLevelName true))
      (Game|OpenLevel(byName) (Utilities|String|StringToName _returnvalue)))))

(event EventBeginPlay
  (bind _stamina (Variables|Default|GetStamina))
  (bind _experience (Variables|Default|GetExperience))
  (bind _returnvalue (UserInterface|CreateWidget "/Game/Widgets/W_Stats.W_Stats_C"))
  (bind _output_get (Variables|Default|SetStat%20Widget _returnvalue))
  (UserInterface|Viewport|AddtoViewport _output_get 0)
  (CallFunction|ChangeHealth 0.0)
  (Progress|SetPercent (Variables|/Game/Widgets/W_Stats.W_Stats_C|GetStaminaBar (Variables|Default|GetStat%20Widget)) (/ (.z _stamina) (.y _stamina)))
  (Progress|SetPercent (Variables|/Game/Widgets/W_Stats.W_Stats_C|GetXPBar (Variables|Default|GetStat%20Widget)) (/ (.z _experience) (.y _experience))))

(event EventTick
  (params (DeltaSeconds :type Float%20%28single-precision%29)))

(fn ChangeHealth
  (params (By%20amount :type Float%20%28double-precision%29))
  (Variables|Default|SetHealth (Math|Vector|MakeVector (.x (Variables|Default|GetHealth)) (.y (Variables|Default|GetHealth)) (+ (.z (Variables|Default|GetHealth)) By%20amount)))
  (Progress|SetPercent (Variables|/Game/Widgets/W_Stats.W_Stats_C|GetHPBar (Variables|Default|GetStat%20Widget)) (/ (.z (Variables|Default|GetHealth)) (+ (.x (Variables|Default|GetHealth)) (.y (Variables|Default|GetHealth)))))
  (if (<= (.z (Variables|Default|GetHealth)) 0.0)
    (CallFunction|Death)))

(fn SetHealth
  (params (Health%20X :type Float%20%28double-precision%29) (Health%20Y :type Float%20%28double-precision%29) (Health%20Z :type Float%20%28double-precision%29))
  (if (== Health%20X -1.0)
    (LocalVariables|SetMinHealth (.x (Variables|Default|GetHealth)))
    (else
      (LocalVariables|SetMinHealth Health%20X)))
  (if (== Health%20Y -1.0)
    (LocalVariables|SetMaxHealth (.y (Variables|Default|GetHealth)))
    (else
      (LocalVariables|SetMaxHealth Health%20Y)))
  (if (== Health%20Z -1.0)
    (LocalVariables|SetCurrentHealth (.z (Variables|Default|GetHealth)))
    (else
      (LocalVariables|SetCurrentHealth Health%20Z)))
  (Variables|Default|SetHealth (Math|Vector|MakeVector (LocalVariables|GetMinHealth) (LocalVariables|GetMaxHealth) (LocalVariables|GetCurrentHealth)))
  (Progress|SetPercent (Variables|/Game/Widgets/W_Stats.W_Stats_C|GetHPBar (Variables|Default|GetStat%20Widget)) (/ (.z (Variables|Default|GetHealth)) (+ (.x (Variables|Default|GetHealth)) (.y (Variables|Default|GetHealth))))))

(fn ChangeXP
  (params (By%20amount :type Float%20%28double-precision%29))
  (bind _stat_widget (Variables|Default|GetStat%20Widget))
  (bind _xpbar (Variables|/Game/Widgets/W_Stats.W_Stats_C|GetXPBar _stat_widget))
  (Variables|Default|SetExperience (Math|Vector|MakeVector (.x (Variables|Default|GetExperience)) (.y (Variables|Default|GetExperience)) (+ (.z (Variables|Default|GetExperience)) By%20amount)))
  (if (== (/ (.z (Variables|Default|GetExperience)) (.y (Variables|Default|GetExperience))) 1.0) :!label _label
    (Progress|SetPercent _xpbar 0.0)
    (else
      (Development|PrintString (Utilities|String|ToString(Float) (/ (.z (Variables|Default|GetExperience)) (.y (Variables|Default|GetExperience)))))
      (Progress|SetPercent _xpbar (/ (.z (Variables|Default|GetExperience)) (.y (Variables|Default|GetExperience))))
      (Variables|/Game/Widgets/W_Stats.W_Stats_C|SetLevel _stat_widget (Utilities|Text|ToText(Float) (.x (Variables|Default|GetExperience)) "HalfToEven"))))
  (if (>= (.z (Variables|Default|GetExperience)) (.y (Variables|Default|GetExperience)))
    (Variables|Default|SetExperience (Math|Vector|MakeVector (+ (.x (Variables|Default|GetExperience)) 1.0) (.y (Variables|Default|GetExperience)) (- (.z (Variables|Default|GetExperience)) (.y (Variables|Default|GetExperience)))))
    (Variables|Default|SetExperience (Math|Vector|MakeVector (.x (Variables|Default|GetExperience)) (* (.y (Variables|Default|GetExperience)) 2.0) (.z (Variables|Default|GetExperience))))
    (Development|PrintString "LevelUp!")
    (goto _label)
    (elif (< (.z (Variables|Default|GetExperience)) 0.0)
      (Variables|Default|SetExperience (Math|Vector|MakeVector (- (.x (Variables|Default|GetExperience)) 1.0) (.y (Variables|Default|GetExperience)) (.z (Variables|Default|GetExperience))))
      (Variables|Default|SetExperience (Math|Vector|MakeVector (.x (Variables|Default|GetExperience)) (/ (.y (Variables|Default|GetExperience)) 2.0) (.z (Variables|Default|GetExperience))))
      (Variables|Default|SetExperience (Math|Vector|MakeVector (.x (Variables|Default|GetExperience)) (.y (Variables|Default|GetExperience)) (+ (.z (Variables|Default|GetExperience)) (.y (Variables|Default|GetExperience)))))
      (Development|PrintString (Utilities|String|ToString(Vector) (Variables|Default|GetExperience)))
      (if (< (.x (Variables|Default|GetExperience)) 0.0)
        (Variables|Default|SetExperience "0.000000,100.000000,0.000000"))
      (Development|PrintString "LevelDown!")
      (goto _label))))

(fn ChangeStamina)

(fn SetStamina)

(fn SetXP
  (params (NewLevel :type Float%20%28double-precision%29) (NewXPToNextLevel :type Float%20%28double-precision%29) (NewCurrentXP :type Float%20%28double-precision%29))
  (bind _stat_widget (Variables|Default|GetStat%20Widget))
  (if (== NewLevel -1.0)
    (LocalVariables|SetLevel (.x (Variables|Default|GetExperience)))
    (else
      (LocalVariables|SetLevel NewLevel)))
  (if (== NewXPToNextLevel -1.0)
    (LocalVariables|SetXPToNextLevel (.y (Variables|Default|GetExperience)))
    (else
      (LocalVariables|SetXPToNextLevel NewXPToNextLevel)))
  (if (== NewCurrentXP -1.0)
    (LocalVariables|SetCurrentXP (.z (Variables|Default|GetExperience)))
    (else
      (LocalVariables|SetCurrentXP NewCurrentXP)))
  (Variables|Default|SetExperience (Math|Vector|MakeVector (LocalVariables|GetLevel) (LocalVariables|GetXPToNextLevel) (LocalVariables|GetCurrentXP)))
  (Progress|SetPercent (Variables|/Game/Widgets/W_Stats.W_Stats_C|GetXPBar _stat_widget) (/ (.z (Variables|Default|GetExperience)) (.y (Variables|Default|GetExperience))))
  (Variables|/Game/Widgets/W_Stats.W_Stats_C|SetLevel _stat_widget (Utilities|Text|ToText(Float) (.x (Variables|Default|GetExperience)) "HalfToEven")))