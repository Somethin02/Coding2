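; Turret enemy Blueprint that aims at a sensed target and fires bullets at it.
; HandleSight stores the target and starts the attack on successful sensing, and clears the target otherwise.
; Tick rotates the pivot toward the target's position, led by a fixed fraction of its velocity.
; Attack spawns BP_Bullet at BulletSpawn, then re-calls itself after a delay derived from RateOfFire while the target remains valid.
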(event Custom|Attack
  (Variables|Default|GetEnemyTarget
    (:then
      (Game|SpawnActorfromClass "/Game/Blueprints/Enemies/BP_Bullet.BP_Bullet_C" (Transformation|GetWorldTransform (Variables|Default|GetBulletSpawn)) "Undefined" "MultiplyWithRoot" 0 0)
      (Utilities|FlowControl|Delay (/ 6e+01 (Variables|Default|GetRateOfFire)))
      (CallFunction|Attack))
    (:else)))

(event EventBeginPlay)

(event Collision|EventActorBeginOverlap
  (params (OtherActor :type Actor%20Object%20Reference)))

(event EventTick
  (params (DeltaSeconds :type Float%20%28single-precision%29))
  (bind _enemytarget (Variables|Default|GetEnemyTarget)
    (:then
      (Transformation|SetWorldRotation (Variables|Default|GetPivot) (Math|Rotator|FindLookatRotation (Transformation|GetWorldLocation (Variables|Default|GetDefaultSceneRoot)) (+ (Transformation|GetActorLocation _enemytarget) (* (Transformation|GetVelocity (Variables|Default|GetEnemyTarget)) 0.25))) false false))
    (:else)))

(event EventHandleSight
  (params (Target :type Actor%20Object%20Reference) (SuccessfulySensed :type Boolean) (Location :type Vector :default "0, 0, 0"))
  (if SuccessfulySensed
    (Variables|Default|SetEnemyTarget Target)
    (CallFunction|Attack)
    (else
      (Variables|Default|SetEnemyTarget 0))))

(fn ConstructionScript)