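; AI controller for melee enemies that turns perception stimuli into StateTree events and caches its possessed pawn.
; Perception updates from actors not tagged "AI" are routed by sense class display name to sight, hearing or damage handlers.
; Sight sets or clears TargetActor and sends an Attack event in both cases.
; Hearing and damage store the stimulus location as PointOfInterest and send an Investigating event.
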(event OnTargetPerceptionUpdated(AIPerception)
  (params (Actor :type Actor%20Object%20Reference) (Stimulus :type AI%20Stimulus%20Structure))
  (bind (_age _expirationage _strength _stimuluslocation _receiverlocation _tag _bsuccessfullysensed) (Utilities|Struct|BreakAIStimulus Stimulus))
  (bind _returnvalue (Class|AIPerceptionSystem|GetSenseClassforStimulus Stimulus))
  (if (not (Actor|ActorHasTag Actor "AI"))
    (switch string (Utilities|GetClassDisplayName _returnvalue)
      (:AISense_Sight
        (CallFunction|HandleSight _bsuccessfullysensed Actor)
        (Gameplay|StateTree|SendStateTreeEvent (Variables|Default|GetStateTreeAI) (Utilities|Struct|MakeStateTreeEvent "(TagName=\"AI.Event.Attack\")") :!class /Script/GameplayStateTreeModule.StateTreeComponent))
      (:AISense_Hearing
        (CallFunction|HandleSound _stimuluslocation))
      (:AISense_Damage
        (CallFunction|HandleDamage _stimuluslocation)))))

(event EventTick
  (params (DeltaSeconds :type Float%20%28single-precision%29)))

(event EventPossess
  (params (PossessedPawn :type Pawn%20Object%20Reference))
  (Variables|Default|SetPossessed%20Pawn PossessedPawn))

(fn ConstructionScript)

(fn HandleSight
  (params (Sensed :type Boolean) (Target :type Actor%20Object%20Reference))
  (if Sensed
    (Variables|Default|SetTarget%20Actor Target)
    (Development|PrintString "ActorSaved")
    (else
      (Variables|Default|SetTarget%20Actor 0))))

(fn HandleSound
  (params (Location :type Vector))
  (Variables|Default|SetPointOfInterest Location)
  (Gameplay|StateTree|SendStateTreeEvent (Variables|Default|GetStateTreeAI) (Utilities|Struct|MakeStateTreeEvent "(TagName=\"AI.Event.Investigating\")") :!class /Script/GameplayStateTreeModule.StateTreeComponent))

(fn HandleDamage
  (params (PointOfInterest :type Vector))
  (Variables|Default|SetPointOfInterest PointOfInterest)
  (Gameplay|StateTree|SendStateTreeEvent (Variables|Default|GetStateTreeAI) (Utilities|Struct|MakeStateTreeEvent "(TagName=\"AI.Event.Investigating\")") :!class /Script/GameplayStateTreeModule.StateTreeComponent))