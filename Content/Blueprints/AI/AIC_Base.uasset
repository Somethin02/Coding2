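; AIC_Base is a base AI controller that forwards sight perception results to the pawn it possesses.
; It caches the possessed pawn, then on each perception update ignores actors tagged "AI" and switches on the stimulus sense class display name.
; Sight stimuli go through HandleSight, which sends the target and sensed state to the pawn via a HandleSightMessage call with a zero location.
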(event OnTargetPerceptionUpdated(AIPerception)
  (params (Actor :type Actor%20Object%20Reference) (Stimulus :type AI%20Stimulus%20Structure))
  (bind _returnvalue (Class|AIPerceptionSystem|GetSenseClassforStimulus Stimulus))
  (if (not (Actor|ActorHasTag Actor "AI"))
    (switch string (Utilities|GetClassDisplayName _returnvalue)
      (:AISense_Sight
        (CallFunction|HandleSight (.bSuccessfullySensed (Utilities|Struct|BreakAIStimulus Stimulus)) Actor)))))

(event EventTick
  (params (DeltaSeconds :type Float%20%28single-precision%29)))

(event EventPossess
  (params (PossessedPawn :type Pawn%20Object%20Reference))
  (Variables|Default|SetPossessed%20Pawn PossessedPawn))

(fn ConstructionScript)

(fn HandleSight
  (params (Sensed :type Boolean) (Target :type Actor%20Object%20Reference))
  (Class|BPIAIPerceiver|HandleSight(Message) (Variables|Default|GetPossessed%20Pawn) Target Sensed "0, 0, 0"))