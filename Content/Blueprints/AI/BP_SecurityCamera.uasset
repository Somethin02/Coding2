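; BP_SecurityCamera is an AI security camera that detects a target and calls enemies to its location.
; HandleSight stores the sensed state and target, starting an investigation if the camera is in Looking state.
; After a one-second yellow Investigate delay, it either returns to blue Looking or escalates to red Alert.
; Alert repeats each second, sending every BP_Enemy to the target's position, and drops to Investigate once sight is lost.
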(event Custom|Investigate
  (Rendering|Material|SetMaterial (Variables|Default|GetStaticMesh) 0 "/Game/SimpleMaterials/MI_Yellow.MI_Yellow")
  (Utilities|FlowControl|Delay 1.0)
  (if (Variables|Default|GetPlayerCurrentlySensed)
    (CallFunction|Alert)
    (else
      (CallFunction|Looking))))

(event Custom|Alert
  (if (Variables|Default|GetPlayerCurrentlySensed)
    (bind _outactors (Actor|GetAllActorsOfClass "/Game/Blueprints/Enemies/BP_Enemy.BP_Enemy_C"))
    (for _array_element _outactors
      (Default|GotoSecurityPoint _array_element (Transformation|GetActorLocation (Variables|Default|GetTarget))))
    (Variables|Default|SetCamState "NewEnumerator2")
    (Rendering|Material|SetMaterial (Variables|Default|GetStaticMesh) 0 "/Game/SimpleMaterials/MI_Red.MI_Red")
    (Utilities|FlowControl|Delay 1.0)
    (CallFunction|Alert)
    (else
      (CallFunction|Investigate))))

(event Custom|Looking
  (Variables|Default|SetCamState "NewEnumerator0")
  (Rendering|Material|SetMaterial (Variables|Default|GetStaticMesh) 0 "/Game/SimpleMaterials/MI_Blue.MI_Blue"))

(event EventBeginPlay)

(event Collision|EventActorBeginOverlap
  (params (OtherActor :type Actor%20Object%20Reference)))

(event EventTick
  (params (DeltaSeconds :type Float%20%28single-precision%29))
  (if (Variables|Default|GetPlayerCurrentlySensed)
    (Development|PrintText "I see you")))

(event EventHandleSight
  (params (Target :type Actor%20Object%20Reference) (SuccessfulySensed :type Boolean) (Location :type Vector :default "0, 0, 0"))
  (Variables|Default|SetPlayerCurrentlySensed SuccessfulySensed)
  (Variables|Default|SetTarget Target)
  (switch Utilities|FlowControl|Switch|SwitchonE_CamState (Variables|Default|GetCamState)
    (:NewEnumerator0
      (CallFunction|Investigate))))

(fn ConstructionScript)