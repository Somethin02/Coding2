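; BPC_Interact is a first-person character component that lets the player inspect and open doors.
; On BeginPlay it caches the camera of the owning BP_FirstPersonCharacter.
; A left mouse press line-traces along the camera's forward vector up to LookDistance, with debug drawing.
; Any hit prints the actor's name and distance and spawns an arrow decal, then a cast to BP_Door triggers TryToOpenDoor.
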(event Custom|Try%20to%20interact
  (bind _first_person_camera (Variables|Default|GetFirst%20Person%20Camera))
  (bind _returnvalue (Transformation|GetWorldLocation _first_person_camera))
  (bind (_outhit _returnvalue_2) (Collision|LineTraceByChannel _returnvalue (+ _returnvalue (* (Math|Vector|GetForwardVector _first_person_camera) (Variables|Default|GetLookDistance))) "TraceTypeQuery1" false 0 "ForDuration"))
  (if _returnvalue_2
    (Development|PrintString (Utilities|String|ToString(Text) (Utilities|Text|FormatText "Look at this, {name}, Bro! It's {distance} cm away!" (Utilities|GetDisplayName (.HitActor (Collision|BreakHitResult _outhit))) (.Distance (Collision|BreakHitResult _outhit)))))
    (Rendering|Decal|SpawnDecalatLocation "/Engine/VREditor/UI/ArrowMaterial.ArrowMaterial" "10.000000,10.000000,10.000000" (.Location (Collision|BreakHitResult _outhit)) "-90.000000,0.000000,0.000000" 0.0)
    (bind _asbp_door (Utilities|Casting|CastToBP_Door (.HitActor (Collision|BreakHitResult _outhit))))
    (Default|TrytoOpenDoor _asbp_door)))

(event EventBeginPlay
  (bind _asbp_first_person_character (Utilities|Casting|CastToBP_FirstPersonCharacter (Components|GetOwner)))
  (Variables|Default|SetFirst%20Person%20Camera (Variables|/Game/FirstPerson/Blueprints/BP_FirstPersonCharacter.BP_FirstPersonCharacter_C|GetFirstPersonCamera _asbp_first_person_character)))

(event Input|MouseEvents|LeftMouseButton
  (params (Key :type Key%20Structure :default "None"))
  (:Pressed
    (CallFunction|TrytoInteract)))