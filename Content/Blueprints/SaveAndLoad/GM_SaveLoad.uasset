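; Game mode that loads and saves the first-person player's progress through an SG_Player save slot.
; On BeginPlay it restores belt and backpack inventories, then retries each tick until the stats widget is valid before applying non-zero health, XP and last transform.
; Without an existing save it creates a fresh save object.
; SavePlayer copies the passed-in inventory, transform, HP and XP into that object and writes it to the slot.
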(event Custom|LoadPlayer
  ;[0.15 0.15 0.15 0.5] FileManagement
  (bind _returnvalue (SaveGame|DoesSaveGameExist (Variables|Default|GetSlot%20Name)))
  (if _returnvalue
    (bind _returnvalue_2 (SaveGame|LoadGamefromSlot (Variables|Default|GetSlot%20Name)))
    (bind _assg_player (Utilities|Casting|CastToSG_Player _returnvalue_2))
    (Variables|Default|SetPlayerSave _assg_player)
    (bind _asbp_first_person_character (Utilities|Casting|CastToBP_FirstPersonCharacter (Game|GetPlayerCharacter 0)))
    (Default|SetInventory (Variables|/Game/FirstPerson/Blueprints/BP_FirstPersonCharacter.BP_FirstPersonCharacter_C|GetInv_Belt _asbp_first_person_character) (Variables|/Game/Blueprints/SaveAndLoad/SG_Player.SG_Player_C|GetBelt (Variables|Default|GetPlayerSave)))
    (Default|SetInventory (Variables|/Game/FirstPerson/Blueprints/BP_FirstPersonCharacter.BP_FirstPersonCharacter_C|GetInv_Backpack _asbp_first_person_character) (Variables|/Game/Blueprints/SaveAndLoad/SG_Player.SG_Player_C|GetInventory (Variables|Default|GetPlayerSave)))
    (Utilities|IsValid (Variables|/Game/Blueprints/BPC_PlayerStats.BPC_PlayerStats_C|GetStat%20Widget (Variables|/Game/FirstPerson/Blueprints/BP_FirstPersonCharacter.BP_FirstPersonCharacter_C|GetBPC_PlayerStats _asbp_first_person_character)) :!label _label
      (:Is%20Valid
        (if (Class|KismetMathLibrary|EqualExactlyVectorVector (Variables|/Game/Blueprints/SaveAndLoad/SG_Player.SG_Player_C|GetPlayerHP (Variables|Default|GetPlayerSave)) "0, 0, 0")
          _
          (else
            (Default|SetHealth (Variables|/Game/FirstPerson/Blueprints/BP_FirstPersonCharacter.BP_FirstPersonCharacter_C|GetBPC_PlayerStats _asbp_first_person_character) (.x (Variables|/Game/Blueprints/SaveAndLoad/SG_Player.SG_Player_C|GetPlayerHP (Variables|Default|GetPlayerSave))) (.y (Variables|/Game/Blueprints/SaveAndLoad/SG_Player.SG_Player_C|GetPlayerHP (Variables|Default|GetPlayerSave))) (.z (Variables|/Game/Blueprints/SaveAndLoad/SG_Player.SG_Player_C|GetPlayerHP (Variables|Default|GetPlayerSave))))
            (Development|PrintString "hp set")))
        (if (Class|KismetMathLibrary|EqualExactlyVectorVector (Variables|/Game/Blueprints/SaveAndLoad/SG_Player.SG_Player_C|GetPlayerXP (Variables|Default|GetPlayerSave)) "0, 0, 0")
          _
          (else
            (Default|SetXP (Variables|/Game/FirstPerson/Blueprints/BP_FirstPersonCharacter.BP_FirstPersonCharacter_C|GetBPC_PlayerStats _asbp_first_person_character) (.x (Variables|/Game/Blueprints/SaveAndLoad/SG_Player.SG_Player_C|GetPlayerXP (Variables|Default|GetPlayerSave))) (.y (Variables|/Game/Blueprints/SaveAndLoad/SG_Player.SG_Player_C|GetPlayerXP (Variables|Default|GetPlayerSave))) (.z (Variables|/Game/Blueprints/SaveAndLoad/SG_Player.SG_Player_C|GetPlayerXP (Variables|Default|GetPlayerSave))))
            (Development|PrintString "Hello")))
        (if (not (Class|KismetMathLibrary|EqualExactlyVectorVector (.Location (Math|Transform|BreakTransform (Variables|/Game/Blueprints/SaveAndLoad/SG_Player.SG_Player_C|GetLastPosition (Variables|Default|GetPlayerSave)))) "0, 0, 0"))
          (Transformation|SetWorldTransform (Variables|/Script/Engine.Character|GetCapsuleComponent _asbp_first_person_character) (Variables|/Game/Blueprints/SaveAndLoad/SG_Player.SG_Player_C|GetLastPosition (Variables|Default|GetPlayerSave)) false false)
          (Development|PrintText "INVENTORY")))
      (:Is%20Not%20Valid
        (Development|PrintString "not valid")
        (Utilities|FlowControl|DelayUntilNextTick)
        (goto _label)))
    (else
      (bind _returnvalue_3 (SaveGame|CreateSaveGameObject "/Game/Blueprints/SaveAndLoad/SG_Player.SG_Player_C"))
      (Variables|Default|SetPlayerSave _returnvalue_3))))

(event Custom|SavePlayer
  (params (Belt :type Array%20of%20E_Item%20Enums :default "NewEnumerator0") (Inventory :type Array%20of%20E_Item%20Enums :default "NewEnumerator0") (LastPosition :type Transform) (HP :type Vector) (XP :type Vector))
  (bind _playersave (Variables|Default|GetPlayerSave))
  (Variables|/Game/Blueprints/SaveAndLoad/SG_Player.SG_Player_C|SetBelt _playersave Belt)
  (Variables|/Game/Blueprints/SaveAndLoad/SG_Player.SG_Player_C|SetInventory _playersave Inventory)
  (Variables|/Game/Blueprints/SaveAndLoad/SG_Player.SG_Player_C|SetLastPosition _playersave LastPosition)
  (Variables|/Game/Blueprints/SaveAndLoad/SG_Player.SG_Player_C|SetPlayerHP _playersave HP)
  (Variables|/Game/Blueprints/SaveAndLoad/SG_Player.SG_Player_C|SetPlayerXP _playersave XP)
  (bind _returnvalue (SaveGame|SaveGametoSlot (Variables|Default|GetPlayerSave) (Variables|Default|GetSlot%20Name)))
  (if _returnvalue
    (Development|PrintText "Yippe")
    (else
      (Development|PrintText "Damn, not here"))))

(event EventBeginPlay
  (Development|PrintText "GameMode loaded" true true "(R=1.000000,G=0.888801,B=0.000000,A=1.000000)" 5.0)
  (CallFunction|LoadPlayer))

(event EventTick
  (params (DeltaSeconds :type Float%20%28single-precision%29)))

(fn ConstructionScript)