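; BP_NextLevel is a level-transition trigger that saves player progress and opens a destination level.
; When BP_FirstPersonCharacter overlaps its Box, it passes the belt and backpack inventories, health and experience to GM_SaveLoad's Save, along with the LoadingPlacement component's transform as the last position.
; It then opens the Destination level by object reference.
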(event OnComponentBeginOverlap(Box)
  (params (OverlappedComponent :type Primitive%20Component%20Object%20Reference) (OtherActor :type Actor%20Object%20Reference) (OtherComp :type Primitive%20Component%20Object%20Reference) (OtherBodyIndex :type Integer) (bFromSweep :type Boolean) (SweepResult :type Hit%20Result%20Structure%20%28by%20ref%29))
  (bind _asbp_first_person_character (Utilities|Casting|CastToBP_FirstPersonCharacter OtherActor))
  (bind _asgm_save_load (Utilities|Casting|CastToGM_SaveLoad (Game|GetGameMode)))
  (Default|Save _asgm_save_load (Variables|/Game/Blueprints/BPC_Inventory.BPC_Inventory_C|GetEnumInv (Variables|/Game/FirstPerson/Blueprints/BP_FirstPersonCharacter.BP_FirstPersonCharacter_C|GetInv_Belt _asbp_first_person_character)) (Variables|/Game/Blueprints/BPC_Inventory.BPC_Inventory_C|GetEnumInv (Variables|/Game/FirstPerson/Blueprints/BP_FirstPersonCharacter.BP_FirstPersonCharacter_C|GetInv_Backpack _asbp_first_person_character)) (Transformation|GetWorldTransform (Variables|Default|GetLoadingPlacement)) (Variables|/Game/Blueprints/BPC_PlayerStats.BPC_PlayerStats_C|GetHealth (Variables|/Game/FirstPerson/Blueprints/BP_FirstPersonCharacter.BP_FirstPersonCharacter_C|GetBPC_PlayerStats _asbp_first_person_character)) (Variables|/Game/Blueprints/BPC_PlayerStats.BPC_PlayerStats_C|GetExperience (Variables|/Game/FirstPerson/Blueprints/BP_FirstPersonCharacter.BP_FirstPersonCharacter_C|GetBPC_PlayerStats _asbp_first_person_character)))
  (Game|OpenLevel(byObjectReference) (Variables|Default|GetDestination)))

(event EventBeginPlay)

(event Collision|EventActorBeginOverlap
  (params (OtherActor :type Actor%20Object%20Reference)))

(event EventTick
  (params (DeltaSeconds :type Float%20%28single-precision%29)))

(fn ConstructionScript)