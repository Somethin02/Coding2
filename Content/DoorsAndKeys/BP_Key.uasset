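; Key actor that can be picked up, dropped and used, with use destroying it.
; PickUp stores the owner and disables box collision; Drop clears KeyOwner's held item, restores collision and physics, and applies a fixed impulse.
; Use clears the held item, calls TryToDrop on the stored owner and destroys the key.
; KeyOwner is never assigned a holder here, and the logic adding AssignedDoor to the player's HeldKeys is disconnected.
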(event EventBeginPlay)

(event Collision|EventActorBeginOverlap
  (params (OtherActor :type Actor%20Object%20Reference)))

(event EventUse
  (Variables|/Game/Blueprints/BPC_Interact.BPC_Interact_C|SetHeldItem (Variables|Default|GetKeyOwner) 0)
  (Default|TrytoDrop (Variables|Default|GetOwner_0))
  (Actor|DestroyActor))

(event EventAltUse)

(event EventDrop
  (bind _box (Variables|Default|GetBox))
  (Variables|/Game/Blueprints/BPC_Interact.BPC_Interact_C|SetHeldItem (Variables|Default|GetKeyOwner) 0)
  (Collision|SetCollisionEnabled (Variables|Default|GetBox) "QueryAndPhysics")
  (Physics|SetSimulatePhysics _box true)
  (Physics|AddImpulse _box "2000.000000,0.000000,50.000000" "None" true))

(event EventTick
  (params (DeltaSeconds :type Float%20%28single-precision%29)))

(fn ConstructionScript)

(fn PickUp
  (params (Owner :type BPC%20Interact%20Object%20Reference))
  (Variables|Default|SetOwner_0 Owner)
  (Collision|SetCollisionEnabled (Variables|Default|GetBox) "NoCollision"))