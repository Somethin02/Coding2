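; BP_Door is a key-locked swinging door that opens when the first-person character enters its trigger box.
; On overlap it searches the character's HeldKeys for itself, either reporting it locked or unlocking it once, with sounds for each state.
; A timeline lerps the pivot 100 degrees in yaw, disabling door collision until finished.
; Leaving the box reverses the timeline if the door is unlocked.
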(event OnComponentBeginOverlap(Box)
  (params (OverlappedComponent :type Primitive%20Component%20Object%20Reference) (OtherActor :type Actor%20Object%20Reference) (OtherComp :type Primitive%20Component%20Object%20Reference) (OtherBodyIndex :type Integer) (bFromSweep :type Boolean) (SweepResult :type Hit%20Result%20Structure%20%28by%20ref%29))
  (bind _asbp_first_person_character (Utilities|Casting|CastToBP_FirstPersonCharacter OtherActor))
  (if (== (Utilities|Array|FindItem (Variables|/Game/FirstPerson/Blueprints/BP_FirstPersonCharacter.BP_FirstPersonCharacter_C|GetHeldKeys _asbp_first_person_character) self) -1)
    (Development|PrintString "Door Locked")
    (Audio|PlaySoundatLocation "/Game/Audio/DoorLocked.DoorLocked" (Transformation|GetWorldLocation (Variables|Default|GetDoor)) "0, 0, 0" 1.0 1.0 0.0 0 0 0 0)
    (elif (Variables|Default|GetUnlocked)
      (CallFunction|OpenDoor)
      (else
        (Variables|Default|SetUnlocked true)
        (Audio|PlaySoundatLocation "/Game/Audio/DoorUnlock.DoorUnlock" (Transformation|GetWorldLocation (Variables|Default|GetDoor)) "0, 0, 0" 1.0 1.0 0.0 0 0 0 0)
        (CallFunction|OpenDoor)))))

(event OnComponentEndOverlap(Box)
  (params (OverlappedComponent :type Primitive%20Component%20Object%20Reference) (OtherActor :type Actor%20Object%20Reference) (OtherComp :type Primitive%20Component%20Object%20Reference) (OtherBodyIndex :type Integer))
  (Utilities|Casting|CastToBP_FirstPersonCharacter OtherActor)
  (if (Variables|Default|GetUnlocked)
    (bind _newtrack_0 (Timeline|Timeline Reverse)
      (:Update
        (Transformation|SetWorldRotation (Variables|Default|GetRotatePoint) (Math|Rotator|Lerp(Rotator) (Variables|Default|GetDoorStartRot) (Variables|Default|GetDoorEndRot) _newtrack_0) false false))
      (:Finished
        (Collision|SetCollisionEnabled (Variables|Default|GetDoor) "QueryAndPhysics")))))

(event Custom|OpenDoor
  (Audio|PlaySoundatLocation "/Game/Audio/DoorOpen.DoorOpen" (Transformation|GetWorldLocation (Variables|Default|GetDoor)) "0, 0, 0" 1.0 1.0 0.0 0 0 0 0)
  (Collision|SetCollisionEnabled (Variables|Default|GetDoor) "NoCollision")
  (bind _newtrack_0 (Timeline|Timeline Play)
    (:Update
      (Transformation|SetWorldRotation (Variables|Default|GetRotatePoint) (Math|Rotator|Lerp(Rotator) (Variables|Default|GetDoorStartRot) (Variables|Default|GetDoorEndRot) _newtrack_0) false false))
    (:Finished
      (Collision|SetCollisionEnabled (Variables|Default|GetDoor) "QueryAndPhysics"))))

(event EventBeginPlay
  (bind _rotatepoint (Variables|Default|GetRotatePoint))
  (bind _returnvalue (Transformation|GetWorldRotation _rotatepoint))
  (Variables|Default|SetDoorEndRot (Math|Rotator|MakeRotator (.roll _returnvalue) (.pitch _returnvalue) (+ (.yaw _returnvalue) 1e+02)))
  (Variables|Default|SetDoorStartRot (Transformation|GetWorldRotation (Variables|Default|GetRotatePoint))))

(event Collision|EventActorBeginOverlap
  (params (OtherActor :type Actor%20Object%20Reference)))

(event EventTick
  (params (DeltaSeconds :type Float%20%28single-precision%29)))

(fn ConstructionScript)